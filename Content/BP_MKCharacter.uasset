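; BP_MKCharacter is a modular character with swappable weapon mesh and melee hit detection.
; Weapon, Armor, Head and Shoulder meshes follow the main Mesh through master pose, and ChangeCloth_Event swaps the weapon mesh.
; TriggerWeapon starts a fast looping timer that line-traces between the weapon's bottom and top sockets with debug drawing, applying fixed damage on each trace until StopTriggerWeapon clears it.
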(event `self.ReceiveBeginPlay`
  (`SkinnedMeshComponent.SetLeaderPoseComponent` (`self.Weapon`) (`self.Mesh`) true)
  (`SkinnedMeshComponent.SetLeaderPoseComponent` (`self.Armor`) (`self.Mesh`) true)
  (`SkinnedMeshComponent.SetLeaderPoseComponent` (`self.Head`) (`self.Mesh`) true)
  (`SkinnedMeshComponent.SetLeaderPoseComponent` (`self.Shoulder`) (`self.Mesh`) true))

(event `ChangeCloth_Event`
  (`SkinnedMeshComponent.SetSkinnedAssetAndUpdate` (`self.Weapon`) "/Game/Models/Equipments/Weapon2/weapon_2.weapon_2" true))

(event `TriggerWeapon`
  (bind _returnvalue (`KismetSystemLibrary.K2_SetTimerDelegate` (delegate `WeaponLineTrace`) 0.01 true))
  (set `self.WeaponTriggerHandler` _returnvalue))

(event `WeaponLineTrace`
  (bind _weapon (`self.Weapon`))
  (bind _outhit (`KismetSystemLibrary.LineTraceSingle` :`Start` (`SceneComponent.GetSocketLocation` _weapon "weapon_bot_05") :`End` (`SceneComponent.GetSocketLocation` _weapon "weapon_top_05") :`TraceChannel` "TraceTypeQuery2" :`DrawDebugType` "ForDuration"))
  (`GameplayStatics.ApplyDamage` (`.HitActor` (`GameplayStatics.BreakHitResult` _outhit)) 40.0))

(event `StopTriggerWeapon`
  (`KismetSystemLibrary.K2_ClearAndInvalidateTimerHandle` (`self.WeaponTriggerHandler`)))

(fn `UserConstructionScript`)