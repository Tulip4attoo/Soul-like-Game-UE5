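; BP_Character is a character Blueprint built from modular Weapon, Armor, Head and Shoulder meshes.
; On BeginPlay those parts take the main Mesh as master pose component, so they follow its animation.
; A timed test sequence then prints a message, swaps the Weapon to another skeletal mesh, and briefly disables movement before restoring walking.
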(event `self.ReceiveBeginPlay`
  (`SkinnedMeshComponent.SetLeaderPoseComponent` (`self.Weapon`) (`self.Mesh`) true)
  (`SkinnedMeshComponent.SetLeaderPoseComponent` (`self.Armor`) (`self.Mesh`) true)
  (`SkinnedMeshComponent.SetLeaderPoseComponent` (`self.Head`) (`self.Mesh`) true)
  (`SkinnedMeshComponent.SetLeaderPoseComponent` (`self.Shoulder`) (`self.Mesh`) true)
  (`KismetSystemLibrary.Delay` 5.0)
  (`KismetSystemLibrary.PrintString` "Hello")
  (`SkinnedMeshComponent.SetSkinnedAssetAndUpdate` (`self.Weapon`) "/Game/Models/Equipments/Weapon2/weapon_2.weapon_2" true)
  (`CharacterMovementComponent.SetMovementMode` (`self.CharacterMovement`) "MOVE_None" 0)
  (`KismetSystemLibrary.Delay` 2.0)
  (`CharacterMovementComponent.SetMovementMode` (`self.CharacterMovement`) "MOVE_Walking" 0))

(fn `UserConstructionScript`)