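; BP_MeleeMinion is a melee minion character that reacts to damage with hit and death montages.
; AnyDamage passes damage to the Attribute object's ApplyHealthChange, prints debug output, then plays death or hit based on remaining health.
; A DoOnce gate ignores further damage until a delay matching the hit montage's length ends, and stays closed after death.
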(event `self.ReceiveAnyDamage`
  (params (Damage :type "Float (single-precision)") (DamageType :type "DamageType Object Reference") (InstigatedBy :type "Controller Object Reference") (DamageCauser :type "Actor Object Reference"))
  (bind _attribute (`self.Attribute`))
  (bind _health (`AttributeComponent.Health` _attribute))
  (`/Engine/EditorBlueprintResources/StandardMacros.DoOnce` false :!label _label
    (:`Completed`
      (bind _result (`/Engine/EditorBlueprintResources/StandardMacros.NegateFloat` Damage)
        (:`  `
          (`AttributeComponent.ApplyHealthChange` _attribute _result)
          (`KismetSystemLibrary.PrintString` (`KismetStringLibrary.Conv_DoubleToString` _health))
          (if (<= _health 0.0)
            (`KismetSystemLibrary.PrintString` "1")
            (`self.PlayAnimMontage` "/Game/Animations/AM_MeleeMinion_Death.AM_MeleeMinion_Death")
            (else
              (`KismetSystemLibrary.PrintString` "2")
              (bind _returnvalue (`self.PlayAnimMontage` "/Game/Animations/AM_MeleeMinion_Hit.AM_MeleeMinion_Hit"))
              (`KismetSystemLibrary.Delay` _returnvalue)
              (goto _label :!via `Reset`))))))))

(fn `UserConstructionScript`)