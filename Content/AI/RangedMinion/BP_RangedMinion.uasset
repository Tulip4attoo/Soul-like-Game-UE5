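; Ranged minion AI enemy that handles taking damage and dying.
; Damage sets the player pawn as the blackboard target, lowers Health and adds a new health bar widget to the viewport on every hit.
; Surviving hits play a montage and briefly disable movement.
; Death plays a montage, removes the TargetingHelper socket, detaches the controller, then switches the mesh to ragdoll physics before delayed destruction.
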(event `self.ReceiveBeginPlay`
  (set `self.Health` (`self.HealthMax`)))

(event `self.ReceiveAnyDamage`
  (params (Damage :type "Float (single-precision)") (DamageType :type "DamageType Object Reference") (InstigatedBy :type "Controller Object Reference") (DamageCauser :type "Actor Object Reference"))
  (`BlackboardComponent.SetValueAsObject` (`AIBlueprintHelperLibrary.GetBlackboard` null) (`self.TargetActor`) (`GameplayStatics.GetPlayerPawn` 0))
  (set `self.Health` (- (`self.Health`) Damage))
  (bind _returnvalue (`|CreateWidget` "/Game/Widgets/UMG_RangedEnemyHealthBar.UMG_RangedEnemyHealthBar_C" null self))
  (`UserWidget.AddToViewport` _returnvalue 0)
  (bind _output_get (set `self.IsAlive` (> (`self.Health`) 0.0)))
  (if _output_get
    (`CharacterMovementComponent.DisableMovement` (`self.CharacterMovement`))
    (`self.PlayAnimMontage` "/Game/Animations/AM_RangedMinion_Hit.AM_RangedMinion_Hit")
    (`KismetSystemLibrary.Delay` 0.2)
    (`CharacterMovementComponent.SetMovementMode` (`self.CharacterMovement`) "MOVE_Walking" 0)
    (else
      (`self.PlayAnimMontage` "/Game/Animations/AM_RangedMinion_Death.AM_RangedMinion_Death")
      (`TargetingHelperComponent.RemoveSocket` (`self.TargetingHelper`) "None")
      (`PrimitiveComponent.SetCollisionProfileName` (`self.Mesh`) "Ragdoll" false)
      (`self.DetachFromControllerPendingDestroy`)
      (`KismetSystemLibrary.Delay` 0.5)
      (`SkeletalMeshComponent.SetAllBodiesSimulatePhysics` (`self.Mesh`) true)
      (`KismetSystemLibrary.Delay` 10.0)
      (`self.K2_DestroyActor`))))

(fn `UserConstructionScript`)