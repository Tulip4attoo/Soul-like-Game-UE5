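; BP_MeleeMinion is a melee AI enemy character that deals damage with two weapons and can be hurt and killed.
; Trigger and stop events for each weapon run looping timers that line trace between trail sockets, applying damage to hit actors on every tick, with debug drawing on.
; Incoming damage lowers Health and plays a hit montage, or on death a death montage, delayed ragdoll, controller detach and destruction.
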(event `TriggerLeftWeapon`
  (bind _returnvalue (`KismetSystemLibrary.K2_SetTimerDelegate` (delegate `LeftWeaponLineTrace`) 0.01 true))
  (set `self.LeftWeaponTriggerHandler` _returnvalue))

(event `LeftWeaponLineTrace`
  (bind _mesh (`self.Mesh`))
  (bind _outhit (`KismetSystemLibrary.LineTraceSingle` :`Start` (`SceneComponent.GetSocketLocation` _mesh "FX_Trail_01_L") :`End` (`SceneComponent.GetSocketLocation` _mesh "FX_Trail_02_L") :`TraceChannel` "TraceTypeQuery2" :`DrawDebugType` "ForDuration"))
  (`GameplayStatics.ApplyDamage` (`.HitActor` (`GameplayStatics.BreakHitResult` _outhit)) 40.0))

(event `StopTriggerLeftWeapon`
  (`KismetSystemLibrary.K2_ClearAndInvalidateTimerHandle` (`self.LeftWeaponTriggerHandler`)))

(event `TriggerRightWeapon`
  (bind _returnvalue (`KismetSystemLibrary.K2_SetTimerDelegate` (delegate `RightWeaponLineTrace`) 0.01 true))
  (set `self.RightWeaponTriggerHandler` _returnvalue))

(event `RightWeaponLineTrace`
  (bind _mesh (`self.Mesh`))
  (bind _outhit (`KismetSystemLibrary.LineTraceSingle` :`Start` (`SceneComponent.GetSocketLocation` _mesh "FX_Trail_01_R") :`End` (`SceneComponent.GetSocketLocation` _mesh "FX_Trail_02_R") :`TraceChannel` "TraceTypeQuery2" :`DrawDebugType` "ForDuration"))
  (`GameplayStatics.ApplyDamage` (`.HitActor` (`GameplayStatics.BreakHitResult` _outhit)) 40.0))

(event `StopTriggerRightWeapon`
  (`KismetSystemLibrary.K2_ClearAndInvalidateTimerHandle` (`self.RightWeaponTriggerHandler`)))

(event `self.ReceiveAnyDamage`
  (params (Damage :type "Float (single-precision)") (DamageType :type "DamageType Object Reference") (InstigatedBy :type "Controller Object Reference") (DamageCauser :type "Actor Object Reference"))
  (bind _output_get (set `self.Health` (- (`self.Health`) Damage)))
  (`KismetSystemLibrary.PrintString` (`KismetStringLibrary.Conv_DoubleToString` _output_get))
  (bind _output_get_2 (set `self.IsAlive` (> (`self.Health`) 0.0)))
  (if _output_get_2
    (`self.PlayAnimMontage` "/Game/Animations/AM_MeleeMinion_Hit.AM_MeleeMinion_Hit")
    (else
      (`self.PlayAnimMontage` "/Game/Animations/AM_MeleeMinion_Death.AM_MeleeMinion_Death")
      (`PrimitiveComponent.SetCollisionProfileName` (`self.Mesh`) "Ragdoll" false)
      (`KismetSystemLibrary.Delay` 0.5)
      (`SkeletalMeshComponent.SetAllBodiesSimulatePhysics` (`self.Mesh`) true)
      (`self.DetachFromControllerPendingDestroy`)
      (`KismetSystemLibrary.Delay` 10.0)
      (`self.K2_DestroyActor`))))

(fn `UserConstructionScript`)